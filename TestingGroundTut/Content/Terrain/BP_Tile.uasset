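; BP_Tile is a terrain segment for an infinite terrain mode that chains tiles as the player moves through them.
; A trigger opens the blocking wall while the player overlaps it, then closes it on exit and asks GM_InfiniteTerrain to spawn another tile.
; The wall's collision and red or green material switch together.
; A second trigger destroys the tile, and GetAttachLocation exposes the AttachPoint transform.
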(event `self.ReceiveBeginPlay`)

(event `self.WallBlockTriggerSpace.OnComponentBeginOverlap`
  (params (OverlappedComponent :type "PrimitiveComponent Object Reference") (OtherActor :type "Actor Object Reference") (OtherComp :type "PrimitiveComponent Object Reference") (OtherBodyIndex :type Integer) (bFromSweep :type Boolean) (SweepResult :type "HitResult Structure (by ref)"))
  (if (== OtherActor (`GameplayStatics.GetPlayerPawn` 0))
    (`self.ToggleBlockingCollision` false)))

(event `self.WallBlockTriggerSpace.OnComponentEndOverlap`
  (params (OverlappedComponent :type "PrimitiveComponent Object Reference") (OtherActor :type "Actor Object Reference") (OtherComp :type "PrimitiveComponent Object Reference") (OtherBodyIndex :type Integer))
  (if (== OtherActor (`GameplayStatics.GetPlayerPawn` 0))
    (`self.ToggleBlockingCollision` true)
    (bind _asgm_infinite_terrain (cast `/Game/GM_InfiniteTerrain` (`GameplayStatics.GetGameMode`)))
    (`/Game/GM_InfiniteTerrain.SpawnTile` _asgm_infinite_terrain)))

(event `self.DestroyTileTriggerSpace.OnComponentBeginOverlap`
  (params (OverlappedComponent :type "PrimitiveComponent Object Reference") (OtherActor :type "Actor Object Reference") (OtherComp :type "PrimitiveComponent Object Reference") (OtherBodyIndex :type Integer) (bFromSweep :type Boolean) (SweepResult :type "HitResult Structure (by ref)"))
  (if (== OtherActor (`GameplayStatics.GetPlayerPawn` 0))
    (`self.K2_DestroyActor`)))

(fn `GetAttachLocation`
  (returns (AttachTransform :type "Transform Structure"))
  (return (`SceneComponent.K2_GetComponentToWorld` (`self.AttachPoint`))))

(fn `ToggleBlockingCollision`
  (params (CollisionState :type Boolean))
  (bind _blockingwall (`self.BlockingWall`))
  (bind _blockingwall_2 (`self.BlockingWall`))
  (if CollisionState
    (`PrimitiveComponent.SetCollisionEnabled` _blockingwall "QueryAndPhysics")
    (`PrimitiveComponent.SetMaterial` _blockingwall 0 "/Game/Terrain/RedBarrier.RedBarrier")
    (else
      (`PrimitiveComponent.SetCollisionEnabled` _blockingwall_2 "NoCollision")
      (`PrimitiveComponent.SetMaterial` _blockingwall_2 0 "/Game/Terrain/GreenBarrier.GreenBarrier"))))

(fn `UserConstructionScript`)